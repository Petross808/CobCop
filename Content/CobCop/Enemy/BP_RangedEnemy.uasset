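; BP_RangedEnemy is a ranged enemy character that shoots on attack requests and reacts to taking damage.
; TryAttack checks that its Health component is alive and its RangedAttack component can attack, then fires and plays a shoot montage.
; On damage it stops the melee crook montage, not the shoot one, and plays a hurt montage.
; Both montages pick a random start section by converting a random integer to a section name.
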(event `self.ReceiveBeginPlay`
  (`parent.ReceiveBeginPlay`))

(event `self.TryAttack`
  (bind _rangedattack (`self.RangedAttack`))
  (if (and (`/Game/CobCop/Components/CombatSystem/BP_HealthComponent.IsAlive` (`self.Health`)) (`/Game/CobCop/Components/CombatSystem/BP_RangedAttack.CanAttack` _rangedattack))
    (`/Game/CobCop/Components/CombatSystem/BP_RangedAttack.TryAttack` _rangedattack)
    (`self.PlayAnimMontage` "/Game/CobCop/Animations/Crook_Ranged/AM_Crook_Ranged_Shoot.AM_Crook_Ranged_Shoot" 1.0 (`KismetStringLibrary.Conv_StringToName` (`KismetStringLibrary.Conv_IntToString` (`KismetMathLibrary.RandomInteger` 3))))))

(event `self.Health.OnDamageEvent`
  (`self.StopAnimMontage` "/Game/CobCop/Animations/Crook_Melee/AM_Crook_Melee_Melee.AM_Crook_Melee_Melee")
  (`self.PlayAnimMontage` "/Game/CobCop/Animations/Crook_Ranged/AM_Crook_Ranged_Hurt.AM_Crook_Ranged_Hurt" 1.0 (`KismetStringLibrary.Conv_StringToName` (`KismetStringLibrary.Conv_IntToString` (`KismetMathLibrary.RandomInteger` 2)))))

(fn `UserConstructionScript`
  (`parent.UserConstructionScript`))