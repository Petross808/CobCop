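; Boss enemy that fetches wooden boxes and throws them at the player.
; A rate-limited tick, gated by Activate/Deactivate, sends it to the nearest pickupable BossBox to carry, falling back to melee when none is reachable.
; With a box, it closes to attack range, turns, then launches it with a physics impulse whose vertical aim scales with distance.
; On death it ragdolls, disables contact damage and drops any held box.
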(event `Activate`
  ; Activate
  (set `self.Active` true)
  (`ActorComponent.SetActive` (`self.CharacterMovement`) true false))

(event `Deactivate`
  ; Deactivate
  (set `self.Active` false)
  (set `self.ChasingPlayer` false)
  (`ActorComponent.SetActive` (`self.CharacterMovement`) false false))

(event `self.ReceiveTick`
  (params (DeltaSeconds :type "Float (single-precision)"))
  ; Tick Behaviour
  (if (`self.Active`)
    (`/Game/CobCop/CustomMacros.TickLimiter` 1.0 DeltaSeconds
      (:`Limited Rate`
        (if (`self.HasBox`)
          (if (not (`self.ChasingPlayer`))
            (`self.Follow`))
          (elif (not (`self.GettingBox`))
            (`self.ObtainBox`)))))))

(event `self.ReceiveBeginPlay`
  (bind _character_sounds (`self.Character Sounds`))
  (bind _boss_sounds (`self.Boss Sounds`))
  ; Save Location on Start and begin Wander
  (`|ExecutionSequence`
    (:`then_0`
      (set `self.StartingLocation` (`self.K2_GetActorLocation`))
      (add `/Game/CobCop/Components/CombatSystem/BP_HealthComponent.OnDeath` (`self.Health`) (delegate `Death`)))
    (:`then_1`
      (`AudioParameterControllerInterface.SetFloatParameter` _character_sounds "Voice Pitch Shift" (`self.VoicePitchShift`))
      (`AudioParameterControllerInterface.SetFloatParameter` _character_sounds "Gain" (`self.CharacterSoundsGain`))
      (`AudioParameterControllerInterface.SetFloatParameter` _boss_sounds "Voice Pitch Shift" (`self.VoicePitchShift`))
      (`AudioParameterControllerInterface.SetFloatParameter` _boss_sounds "Gain" (`self.CharacterSoundsGain`)))))

(event `Death`
  (params (`Healt Component` :type "/Game/CobCop/Components/CombatSystem/BP_HealthComponent Object Reference"))
  (bind _heldbox (`self.HeldBox`))
  ; On Death
  (`/Game/CobCop/Components/Ragdoll/RagdollComponent.StartRagdollMode` (`self.Ragdoll`))
  (`ActorComponent.Deactivate` (`self.Contact Damage`))
  (if (`self.HasBox`)
    (`/Engine/EditorBlueprintResources/StandardMacros.IsValid` _heldbox
      (:`Is Valid`
        (`self.K2_DetachFromActor` _heldbox "KeepRelative" "KeepRelative" "KeepRelative")
        (`PrimitiveComponent.SetSimulatePhysics` (`/Game/CobCop/Blueprints_Prefabs/StorageItems/BoxMid.SM_wooden_box4_v8` _heldbox) true)
        (set `self.HeldBox` null)
        (set `self.HasBox` false)))))

(event `ObtainBox`
  ; Obtain Box
  (bind (_valid _box) (`self.GetClosestBox`))
  (if _valid
    (`|AIMoveTo` self (0.0 0.0 0.0) _box 100.0
      (:`then`
        (set `self.GettingBox` true))
      (:`OnSuccess`
        (`self.AttachBox` _box)
        (set `self.GettingBox` false)
        (`AudioParameterControllerInterface.SetTriggerParameter` (`self.Boss Sounds`) "Pickup"))
      (:`OnFail`
        (set `self.GettingBox` false)
        (`self.MeleeFollow`)))
    (else
      (`self.MeleeFollow`))))

(event `AttachBox`
  (params (Box :type "/Game/CobCop/Enemy/BossBox Object Reference"))
  ; Attach Box
  (set `self.HasBox` true)
  (bind _output_get (set `self.HeldBox` Box))
  (set `/Game/CobCop/Enemy/BossBox.Carried` true _output_get)
  (`PrimitiveComponent.SetSimulatePhysics` (`/Game/CobCop/Blueprints_Prefabs/StorageItems/BoxMid.SM_wooden_box4_v8` _output_get) false)
  (bind _returnvalue (`self.K2_AttachToActor` _output_get self "None" "KeepRelative" "KeepRelative" "KeepWorld" false))
  (if _returnvalue
    (`self.K2_SetActorRelativeLocation` _output_get (0.0 0.0 120.0) false true)))

(event `MeleeFollow`
  (bind _meleeattack (`self.MeleeAttack`))
  ; Melee Follow
  (if (not (`self.ChasingPlayer`))
    (`|AIMoveTo` self (0.0 0.0 0.0) (`GameplayStatics.GetPlayerPawn` 0) 75.0
      (:`then`
        (set `self.ChasingPlayer` true))
      (:`OnSuccess`
        (if (and (`/Game/CobCop/Components/CombatSystem/BP_HealthComponent.IsAlive` (`self.Health`)) (`/Game/CobCop/Components/CombatSystem/BP_AttackComponent.CanAttack` _meleeattack))
          (`/Game/CobCop/Components/CombatSystem/BP_AttackComponent.Try Attack` _meleeattack)
          (`/Game/CobCop/Components/CombatSystem/BP_AttackComponent.Attack` _meleeattack))
        (set `self.ChasingPlayer` false :!label _label))
      (:`OnFail`
        (goto _label)))))

(event `Follow`
  ; Follow Player into Attack Range
  (`|AIMoveTo` self (0.0 0.0 0.0) (`GameplayStatics.GetPlayerPawn` 0) (`self.AttackRange`)
    (:`then`
      (set `self.ChasingPlayer` true))
    (:`OnSuccess`
      (`self.TryAttack`)
      (set `self.ChasingPlayer` false :!label _label_2))
    (:`OnFail`
      (goto _label_2))))

(event `LookAtPlayer`
  (bind _returnvalue (`GameplayStatics.GetPlayerPawn` 0))
  (bind (_returnvalue_roll _returnvalue_pitch _returnvalue_yaw) (`KismetMathLibrary.BreakRotator` (`KismetMathLibrary.FindLookAtRotation` (`self.K2_GetActorLocation`) (`self.K2_GetActorLocation` _returnvalue))))
  ; Look at Player
  (`/Engine/EditorBlueprintResources/StandardMacros.IsValid` _returnvalue
    (:`Is Valid`
      (`self.K2_SetActorRotation` (`KismetMathLibrary.MakeRotator` 0.0 0.0 _returnvalue_yaw)))))

(event `TryAttack`
  (bind _heldbox (`self.HeldBox`))
  (bind _sm_wooden_box4_v8 (`/Game/CobCop/Blueprints_Prefabs/StorageItems/BoxMid.SM_wooden_box4_v8` _heldbox))
  ; Throw Box
  (`self.LookAtPlayer`)
  (`KismetSystemLibrary.Delay` 0.5)
  (`/Engine/EditorBlueprintResources/StandardMacros.IsValid` _heldbox
    (:`Is Valid`
      (`self.K2_DetachFromActor` _heldbox "KeepRelative" "KeepRelative" "KeepRelative")
      (`PrimitiveComponent.SetSimulatePhysics` _sm_wooden_box4_v8 true)
      (`PrimitiveComponent.AddImpulse` _sm_wooden_box4_v8 (* (+ (`self.GetActorForwardVector`) (`KismetMathLibrary.MakeVector` 0.0 0.0 (`KismetMathLibrary.Lerp` -1.0 0.25 (/ (`KismetMathLibrary.Vector_Distance` (`self.K2_GetActorLocation`) (`self.K2_GetActorLocation` (`GameplayStatics.GetPlayerPawn` 0))) (`self.AttackRange`))))) 1000.0) "None" true)
      (`PrimitiveComponent.AddAngularImpulseInDegrees` _sm_wooden_box4_v8 (* (`KismetMathLibrary.RandomUnitVector`) 100.0) "None" true)
      (set `/Game/CobCop/Enemy/BossBox.Active` true (`self.HeldBox`))
      (set `self.HeldBox` null)
      (set `self.HasBox` false)
      (`AudioParameterControllerInterface.SetTriggerParameter` (`self.Boss Sounds`) "Throw"))))

(fn `GetClosestBox`
  (returns (Valid :type Boolean) (Box :type "/Game/CobCop/Enemy/BossBox Object Reference"))
  (locals (Found :type Boolean) (ClosestDistance :type "Float (double-precision)") (ClosestBox :type "/Game/CobCop/Enemy/BossBox Object Reference"))
  (bind _outactors (`GameplayStatics.GetAllActorsOfClass` "/Game/CobCop/Enemy/BossBox.BossBox_C"))
  (for _array_element _outactors
    (if (`/Game/CobCop/Enemy/BossBox.IsPickupable` _array_element)
      (if (`local.Found`)
        (bind _returnvalue (`KismetMathLibrary.Vector_DistanceSquared` (`self.K2_GetActorLocation` _array_element) (`self.K2_GetActorLocation`)))
        (if (< _returnvalue (`local.ClosestDistance`))
          (set `local.ClosestBox` _array_element :!label _label)
          (set `local.ClosestDistance` _returnvalue)
          (set `local.Found` true))
        (else
          (goto _label)))))
  (return (`local.Found`) (`local.ClosestBox`)))

(fn `UserConstructionScript`)