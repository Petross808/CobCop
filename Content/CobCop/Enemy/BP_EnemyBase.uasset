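; Base enemy character that wanders near its spawn point, chases pawns it sees or that damage it, and leaves the attack to an empty TryAttack event.
; Wander and Return alternate via AIMoveTo, while Follow moves into attack range and attacks on arrival.
; A chase timer tires the enemy and sends it home until a cooldown or damage resets aggro.
; Tick yaws it toward its target; death triggers ragdoll and disables sensing and contact damage.
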(event `self.ReceiveBeginPlay`
  ; Save Location on Start and begin Wander
  (`AudioParameterControllerInterface.SetFloatParameter` (`self.Character Sounds`) "Voice Pitch Shift" (`self.VoicePitchShift`))
  (set `self.StartingLocation` (`self.K2_GetActorLocation`))
  (set `self.IsTired` false)
  (add `self.OnTakeAnyDamage` (delegate `OnTakeAnyDamage_Event`))
  (`self.Wander`)
  (add `/Game/CobCop/Components/CombatSystem/BP_HealthComponent.OnDeath` (`self.Health`) (delegate `Death`)))

(event `Death`
  (params (`Healt Component` :type "/Game/CobCop/Components/CombatSystem/BP_HealthComponent Object Reference"))
  ; On Death
  (`/Game/CobCop/Components/Ragdoll/RagdollComponent.StartRagdollMode` (`self.Ragdoll`))
  (`ActorComponent.Deactivate` (`self.Contact Damage`))
  (`ActorComponent.Deactivate` (`self.PawnSensing`))
  (`KismetSystemLibrary.Delay` 2.0)
  (`ActorComponent.K2_DestroyComponent` (`self.Character Sounds`)))

(event `OnTakeAnyDamage_Event` :!signature `self.OnTakeAnyDamage`
  (params (DamagedActor :type "Actor Object Reference") (Damage :type "Float (single-precision)") (DamageType :type "DamageType Object Reference") (InstigatedBy :type "Controller Object Reference") (DamageCauser :type "Actor Object Reference"))
  ; Reset Aggro on Damage
  (set `self.IsTired` false)
  (`|ExecutionSequence`
    (:`then_0`
      (goto _label :!via `Reset`))
    (:`then_1`
      (bind _aspawn (cast `Pawn` DamageCauser))
      (`self.Follow` _aspawn))))

(event `self.PawnSensing.OnSeePawn`
  (params (Pawn :type "Pawn Object Reference"))
  ; Follow Player When Spotted
  (`self.OnPlayerSpotted` (`self.BP_Callout`))
  (if (not (`self.IsTired`))
    (`self.Follow` Pawn)))

(event `Follow`
  (params (TargetPawn :type "Pawn Object Reference"))
  ; Follow Player into Attack Range
  (if (not (`/Game/CobCop/Components/Ragdoll/RagdollComponent.IsRagdoll` (`self.Ragdoll`)))
    (`|AIMoveTo` self (0.0 0.0 0.0) TargetPawn (`self.AttackRange`)
      (:`then`
        (set `self.InChase` true)
        (set `self.ChasedPawn` TargetPawn)
        (`/Engine/EditorBlueprintResources/StandardMacros.DoOnce` false :!label _label
          (:`Completed`
            _)))
      (:`OnSuccess`
        (`self.TryAttack`)
        (`KismetSystemLibrary.K2_ClearAndInvalidateTimerHandle` (stale _returnvalue))))
    (bind _returnvalue (`KismetSystemLibrary.K2_SetTimerDelegate` (delegate `LoseAggro`) (`self.MaxChaseTime`)))))

(event `LoseAggro`
  ; Aggro Control
  (set `self.IsTired` true)
  (set `self.InChase` false)
  (`KismetSystemLibrary.K2_SetTimerDelegate` (delegate `ResetAggro`) (`self.AggroCooldown`))
  (`self.Return`))

(event `ResetAggro`
  ; Aggro Control
  (set `self.IsTired` false)
  (goto _label :!via `Reset`))

(event `Return`
  ; Return to Origin
  (if (not (`self.InChase`))
    (`KismetSystemLibrary.Delay` (`self.TimeBeforeReturn`))
    (`|AIMoveTo` self (`self.StartingLocation`) null (`self.WanderDistance`)
      (:`OnSuccess`
        (`KismetSystemLibrary.Delay` (`self.WanderFrequency`))
        (`self.Wander`)))))

(event `Wander`
  ; Wander
  (if (not (`self.InChase`))
    (bind _randomlocation (`NavigationSystemV1.K2_GetRandomLocationInNavigableRadius` (`self.K2_GetActorLocation`) (`self.WanderDistance`) null null))
    (`|AIMoveTo` self _randomlocation null
      (:`OnSuccess`
        _)
      (:`OnFail`
        _))
    (`KismetSystemLibrary.Delay` (`self.WanderFrequency`))
    (`self.Return`)))

(event `self.ReceiveTick`
  (params (DeltaSeconds :type "Float (single-precision)"))
  (bind (_returnvalue_x _returnvalue_y) (`KismetMathLibrary.BreakVector` (`self.K2_GetActorLocation`)))
  (bind _chasedpawn (`self.ChasedPawn`))
  (bind (_returnvalue_x_2 _returnvalue_y_2) (`KismetMathLibrary.BreakVector` (`self.K2_GetActorLocation` _chasedpawn)))
  ; Smooth Rotation in Chase
  (if (and (`self.InChase`) (`KismetSystemLibrary.IsValid` _chasedpawn))
    (`self.K2_SetActorRotation` (`KismetMathLibrary.FindLookAtRotation` (`KismetMathLibrary.MakeVector` _returnvalue_x _returnvalue_y) (`KismetMathLibrary.MakeVector` _returnvalue_x_2 _returnvalue_y_2)))))

(event `InternalAttack`
  ; Attack
  (if (not (`/Game/CobCop/Components/Ragdoll/RagdollComponent.IsRagdoll` (`self.Ragdoll`)))
    (`self.TryAttack`)))

(event `TryAttack`
  ; Attack
)

(fn `UserConstructionScript`)