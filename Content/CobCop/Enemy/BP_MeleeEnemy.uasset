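; BP_MeleeEnemy is a melee crook enemy character that attacks and reacts to damage with animation montages.
; TryAttack checks that the Health component is alive and the MeleeAttack component can attack, then triggers the attack with a montage section picked at random.
; Damage events from Health stop the melee montage and play a randomly chosen hurt section.
; Random integers converted to names select the montage sections, giving animation variety.
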(event `self.TryAttack`
  (bind _melee_attack (`self.Melee Attack`))
  (if (and (`/Game/CobCop/Components/CombatSystem/BP_HealthComponent.IsAlive` (`self.Health`)) (`/Game/CobCop/Components/CombatSystem/BP_AttackComponent.CanAttack` _melee_attack))
    (`/Game/CobCop/Components/CombatSystem/BP_AttackComponent.Try Attack` _melee_attack)
    (`self.PlayAnimMontage` "/Game/CobCop/Animations/Crook_Melee/AM_Crook_Melee_Melee.AM_Crook_Melee_Melee" 1.0 (`KismetStringLibrary.Conv_StringToName` (`KismetStringLibrary.Conv_IntToString` (`KismetMathLibrary.RandomInteger` 4))))))

(event `self.Health.OnDamageEvent`
  (`self.StopAnimMontage` "/Game/CobCop/Animations/Crook_Melee/AM_Crook_Melee_Melee.AM_Crook_Melee_Melee")
  (`self.PlayAnimMontage` "/Game/CobCop/Animations/Crook_Melee/AM_Crook_Melee_Hurt.AM_Crook_Melee_Hurt" 1.0 (`KismetStringLibrary.Conv_StringToName` (`KismetStringLibrary.Conv_IntToString` (`KismetMathLibrary.RandomInteger` 2)))))

(fn `UserConstructionScript`
  (`parent.UserConstructionScript`))