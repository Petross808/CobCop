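; BP_Tony is the Tony enemy in CobCop, a scripted runner that removes itself after a running sequence.
; PlayStartRun plays a one-shot running animation, then stops the mesh and destroys the actor after a fixed delay.
; PlayRun waits briefly, loops a second running animation while AI MoveTo heads to TargetDoor, and destroys the actor on success.
; A failed move has no handling.
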(event `PlayStartRun`
  (bind _mesh (`self.Mesh`))
  (`SkeletalMeshComponent.PlayAnimation` _mesh "/Game/CobCop/Animations/Crook_Tony/Tony_Running_01.Tony_Running_01" false)
  (`KismetSystemLibrary.Delay` 1.7)
  (`SkeletalMeshComponent.Stop` _mesh)
  (`self.K2_DestroyActor`))

(event `PlayRun`
  (bind _mesh (`self.Mesh`))
  (`KismetSystemLibrary.Delay` 1.0)
  (`SkeletalMeshComponent.PlayAnimation` _mesh "/Game/CobCop/Animations/Crook_Tony/Tony_Running_02.Tony_Running_02" true)
  (`|AIMoveTo` self (0.0 0.0 0.0) (`self.TargetDoor`)
    (:`OnSuccess`
      (`SkeletalMeshComponent.Stop` _mesh)
      (`self.K2_DestroyActor`))))

(fn `UserConstructionScript`)