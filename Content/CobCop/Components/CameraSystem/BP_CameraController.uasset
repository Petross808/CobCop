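; Camera controller component that keeps its owner's camera at a set offset, pulling it in when something blocks the way.
; Finds the owner's camera on BeginPlay, then sphere-traces every tick on the Pawn profile toward the offset, ignoring the owner.
; A hit scales the camera's relative offset by hit distance over offset length; otherwise the full offset applies.
; The trace start nudge normalizes the world position rather than the offset direction.
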(event `self.ReceiveBeginPlay`
  (set `self.Camera` (`Actor.GetComponentByClass` (`self.GetOwner`) "/Script/Engine.CameraComponent")))

(event `self.ReceiveTick`
  (params (DeltaSeconds :type "Float (single-precision)"))
  (bind _offset (`self.Offset`))
  (bind _returnvalue (+ (`self.K2_GetComponentLocation`) (`self.SweepStartOffset`)))
  (`|ExecutionSequence`
    (:`then_0`
      (bind (_outhit _returnvalue_2) (`KismetSystemLibrary.SphereTraceSingleByProfile` (+ _returnvalue (* (`KismetMathLibrary.Normal` _returnvalue) (`self.Radius`))) (+ _returnvalue (`self.Offset`)) (`self.Radius`) "Pawn" false (`|MakeArray` (`self.GetOwner`))))
      (if _returnvalue_2
        (`self.K2_SetRelativeLocation` (`self.Camera`) (* (`KismetMathLibrary.SafeDivide` (`.Distance` (`GameplayStatics.BreakHitResult` _outhit)) (`KismetMathLibrary.VSize` _offset)) _offset) false true)
        (else
          (`self.K2_SetRelativeLocation` (`self.Camera`) (`self.Offset`) false true))))))