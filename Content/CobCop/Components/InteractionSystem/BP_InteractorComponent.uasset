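; Actor component that lets its owner find the nearest interactable and trigger it.
; A rate-limited tick sphere-overlaps around the owner and picks the closest actor with a BP_InteractableComponent.
; A screen-space widget component created at BeginPlay moves to that target and shows its prompt text, clearing when none is in range.
; TryInteract repeats the search and calls Interact on the closest component.
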(event `self.ReceiveBeginPlay`
  (bind _returnvalue (`|AddComponentByClass` :`self` (`self.GetOwner`) :`Class` "/Script/UMG.WidgetComponent" :`bManualAttachment` true))
  (`WidgetComponent.SetWidgetSpace` _returnvalue "Screen")
  (`WidgetComponent.SetDrawSize` _returnvalue (300.0 50.0))
  (set `self.WidgetComponent` _returnvalue)
  (bind _returnvalue_2 (`|CreateWidget` "/Game/CobCop/Components/InteractionSystem/W_InteractPrompt.W_InteractPrompt_C"))
  (set `self.Widget` _returnvalue_2))

(event `self.ReceiveTick`
  (params (DeltaSeconds :type "Float (single-precision)"))
  (`/Game/CobCop/CustomMacros.TickLimiter` 0.1 DeltaSeconds
    (:`Limited Rate`
      (bind (_valid_ _closest) (`self.Get Closest Interactable In Range`))
      (`self.Update Interact Widget` _valid_ _closest))))

(event `Try Interact`
  (bind (_valid_ _closest) (`self.Get Closest Interactable In Range`))
  (if _valid_
    (`/Game/CobCop/Components/InteractionSystem/BP_InteractableComponent.Interact` _closest)))

(fn `Get Closest Interactable In Range`
  (returns (`Valid?` :type Boolean) (Closest :type "/Game/CobCop/Components/InteractionSystem/BP_InteractableComponent Object Reference") (Distance :type "Float (double-precision)"))
  (locals (ClosestDistance :type "Float (double-precision)") (Valid :type Boolean) (ClosestComponent :type "/Game/CobCop/Components/InteractionSystem/BP_InteractableComponent Soft Object Reference"))
  (bind _returnvalue (`self.GetOwner`))
  (bind _returnvalue_2 (`Actor.K2_GetActorLocation` _returnvalue))
  (bind _outactors (`KismetSystemLibrary.SphereOverlapActors` _returnvalue_2 (`self.Interact Range`) (`|MakeArray` "ObjectTypeQuery1" "ObjectTypeQuery2" :!type "EObjectTypeQuery Enum") null (`|MakeArray` _returnvalue)))
  (`|ExecutionSequence`
    (:`then_0`
      (goto _label :!via `Reset`))
    (:`then_1`
      (for _array_element _outactors
        (bind _returnvalue_3 (`Actor.GetComponentByClass` _array_element "/Game/CobCop/Components/InteractionSystem/BP_InteractableComponent.BP_InteractableComponent_C"))
        (`/Engine/EditorBlueprintResources/StandardMacros.IsValid` _returnvalue_3
          (:`Is Valid`
            (`/Game/CobCop/CustomMacros.DoFirstOnce` :!label _label
              (:`First`
                (set `local.Valid` true)
                (bind _returnvalue_4 (`KismetMathLibrary.Vector_Distance` (`Actor.K2_GetActorLocation` _array_element) _returnvalue_2))
                (set `local.ClosestDistance` _returnvalue_4 :!label _label_2)
                (set `local.ClosestComponent` (`|ConvertAsset` _returnvalue_3)))
              (:`Always`
                (if (< _returnvalue_4 (`local.ClosestDistance`))
                  (goto _label_2)))))))
      (return (`local.Valid`) (`|ConvertAsset` (`local.ClosestComponent`)) (`local.ClosestDistance`)))))

(fn `Update Interact Widget`
  (params (Valid :type Boolean) (`Closest Interactable` :type "/Game/CobCop/Components/InteractionSystem/BP_InteractableComponent Object Reference"))
  (bind _widget (`self.Widget`))
  (bind _widgetcomponent (`self.WidgetComponent`))
  (bind _lastclosest (`self.LastClosest`))
  (if Valid
    (if (!= `Closest Interactable` _lastclosest)
      (set `self.LastClosest` `Closest Interactable`)
      (set `/Game/CobCop/Components/InteractionSystem/W_InteractPrompt.Text` (`/Game/CobCop/Components/InteractionSystem/BP_InteractableComponent.Get Interact Text` `Closest Interactable`) _widget)
      (`SceneComponent.K2_SetWorldLocation` _widgetcomponent (`/Game/CobCop/Components/InteractionSystem/BP_InteractableComponent.Get Interact Location` `Closest Interactable`) false false)
      (`WidgetComponent.SetWidget` _widgetcomponent _widget))
    (elif (`KismetSystemLibrary.IsValid` _lastclosest)
      (`WidgetComponent.SetWidget` _widgetcomponent null)
      (set `self.LastClosest` null))))