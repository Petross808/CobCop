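; Melee attack component that deals point damage to pawns and physics bodies inside a sphere around itself.
; TryAttack only gates a cooldown, while Attack runs start, a single overlap tick and a short-delayed end.
; An already-hit list, seeded with the owner, prevents repeat hits; a line trace supplies each hit's info.
; A spawned attack mesh toggles collision with the attack and repositions on hits, and starting triggers melee audio.
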(event `self.ReceiveBeginPlay`
  ; Initialize Audio Component
  (set `self.Audio` (`Actor.GetComponentByClass` (`self.GetOwner`) "/Script/Engine.AudioComponent"))
  (bind _returnvalue (`|SpawnActorFromClass` "/Game/CobCop/Components/CombatSystem/BP_AttackMesh.BP_AttackMesh_C" (`KismetMathLibrary.MakeTransform` (0.0 0.0 0.0) (struct) (* (`self.AttackRadius`) (1.0 1.0 0.5))) "AlwaysSpawn" "MultiplyWithRoot" null null))
  (set `self.AttackMesh` _returnvalue)
  (set `self.CanAttack` true))

(event `Try Attack`
  ; Try Attack
  (if (`self.CanAttack`)
    (set `self.CanAttack` false)
    (`KismetSystemLibrary.Delay` (`self.Cooldown`))
    (set `self.CanAttack` true)))

(event `Attack`
  ; Simple Attack Behaviour
  (`self.Start Attack`)
  (`self.Tick Attack`)
  (`KismetSystemLibrary.Delay` 0.1)
  (`self.End Attack`))

(event `Start Attack`
  ; Attack Start
  (set `self.AlreadyHit` (`|MakeArray` (`self.GetOwner`)))
  (set `self.HItboxActive` true)
  (`AudioParameterControllerInterface.SetTriggerParameter` (`self.Audio`) "Melee")
  (`/Game/CobCop/Components/CombatSystem/BP_AttackMesh.StartCollide` (`self.AttackMesh`)))

(event `Tick Attack`
  (bind _attackmesh (`self.AttackMesh`))
  ; Attack Tick
  (if (`self.HItboxActive`)
    (bind _outactors (`KismetSystemLibrary.SphereOverlapActors` (`self.K2_GetComponentLocation`) (`self.AttackRadius`) (`|MakeArray` "ObjectTypeQuery3" "ObjectTypeQuery4" :!type "EObjectTypeQuery Enum") null (`self.AlreadyHit`)))
    (for _array_element _outactors
      (`self.Apply Damage` _array_element)
      (`Actor.K2_SetActorLocationAndRotation` _attackmesh (`self.K2_GetComponentLocation`) (`self.K2_GetComponentRotation`) false false)
      (`Actor.K2_AddActorLocalOffset` _attackmesh (-30.0 0.0 0.0) false false))
    (`KismetArrayLibrary.Array_Append` (`self.AlreadyHit`) _outactors)))

(event `End Attack`
  ; Attack End
  (set `self.HItboxActive` false)
  (`KismetArrayLibrary.Array_Clear` (`self.AlreadyHit`))
  (`/Game/CobCop/Components/CombatSystem/BP_AttackMesh.StopCollide` (`self.AttackMesh`)))

(fn `Apply Damage`
  (params (DamagedActor :type "Actor Object Reference"))
  (bind _returnvalue (`Actor.K2_GetActorLocation` DamagedActor))
  (bind _returnvalue_2 (`self.GetOwner`))
  (bind _returnvalue_3 (`Actor.K2_GetActorLocation` _returnvalue_2))
  (bind _outhit (`KismetSystemLibrary.LineTraceSingleForObjects` _returnvalue_3 _returnvalue (`|MakeArray` "ObjectTypeQuery1" "ObjectTypeQuery2" "ObjectTypeQuery3" :!type "EObjectTypeQuery Enum") false (`|MakeArray` _returnvalue_2)))
  (`GameplayStatics.ApplyPointDamage` DamagedActor (`self.Damage`) (`KismetMathLibrary.Normal` (- _returnvalue _returnvalue_3)) _outhit null (`self.GetOwner`) "/Script/Engine.DamageType"))