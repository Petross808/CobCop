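; Actor component that manages its owner's health, covering damage, healing, death and revival, with dispatchers for each change.
; It binds to the owner's OnTakeAnyDamage, using a DoOnce gate and CanBeDamaged toggle for invincibility frames after each hit.
; Death optionally spawns a corpse and destroys the owner, while Revive restores full health and damageability.
; Hurt and death sounds fire as trigger parameters on the owner's AudioComponent.
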(event `self.ReceiveBeginPlay`
  (bind _returnvalue (`self.GetOwner`))
  ; Register Damage Callback and initialize audio
  (add `Actor.OnTakeAnyDamage` _returnvalue (delegate `TakeDamage`))
  (set `self.AudioComponent` (`Actor.GetComponentByClass` _returnvalue "/Script/Engine.AudioComponent"))
  (if (<= (`self.Health`) 0.0)
    (`KismetSystemLibrary.DelayUntilNextTick`)
    (`self.Death`)))

(event `TakeDamage`
  (params (DamagedActor :type "Actor Object Reference") (Damage :type "Float (single-precision)") (DamageType :type "DamageType Object Reference") (InstigatedBy :type "Controller Object Reference") (DamageCauser :type "Actor Object Reference"))
  (bind _returnvalue (`self.GetOwner`))
  (bind _health (`self.Health`))
  ; Take Damage
  (`/Engine/EditorBlueprintResources/StandardMacros.DoOnce` false :!label _label
    (:`Completed`
      (`self.AddHealthClamped` (* Damage -1.0))
      (`self.OnDamageEvent` self)
      (`self.OnHealthChanged` _health)
      (if (<= _health 0.0)
        (`self.Death`)
        (else
          (`self.PlaySound` "Hurt")
          (set `Actor.bCanBeDamaged` false _returnvalue)
          (`KismetSystemLibrary.Delay` (`self.IFrames`))
          (set `Actor.bCanBeDamaged` true _returnvalue)
          (goto _label :!via `Reset`))))))

(event `ResetTakeDamage`
  ; Take Damage
  (goto _label :!via `Reset`))

(event `Death`
  ; Death
  (`self.OnDeath` self)
  (`self.PlaySound` "Die")
  (set `Actor.bCanBeDamaged` false (`self.GetOwner`))
  (`self.SpawnCorpse`)
  (if (`self.DestroyOnDeath`)
    (`Actor.K2_DestroyActor` (`self.GetOwner`))))

(event `Heal`
  (params (Amount :type "Float (double-precision)"))
  ; Heal
  (`self.AddHealthClamped` Amount)
  (`self.OnHealEvent`)
  (`self.OnHealthChanged` (`self.Health`)))

(event `Revive`
  ; Revive
  (`self.ResetTakeDamage`)
  (set `self.Health` (`self.MaxHealth`))
  (set `Actor.bCanBeDamaged` true (`self.GetOwner`))
  (`self.OnHealthChanged` (`self.Health`)))

(fn `AddHealthClamped`
  (params (Add :type "Float (double-precision)"))
  (set `self.Health` (`KismetMathLibrary.FClamp` (+ Add (`self.Health`)) 0.0 (`self.MaxHealth`))))

(fn `IsAlive`
  (returns (Alive :type Boolean))
  (return (> (`self.Health`) 0.0)))

(fn `PlaySound`
  (params (Name :type Name))
  (bind _audiocomponent (`self.AudioComponent`))
  (`/Engine/EditorBlueprintResources/StandardMacros.IsValid` _audiocomponent
    (:`Is Valid`
      (`AudioParameterControllerInterface.SetTriggerParameter` _audiocomponent Name))))

(fn `SpawnCorpse`
  (bind _corpse (`self.Corpse`))
  (if (`KismetSystemLibrary.IsValidClass` _corpse)
    (`|SpawnActorFromClass` _corpse (`Actor.GetTransform` (`self.GetOwner`)) "Undefined" "MultiplyWithRoot" null null)))