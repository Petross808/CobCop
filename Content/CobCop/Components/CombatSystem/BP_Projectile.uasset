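; BP_Projectile is a combat projectile that deals point damage on its first impact with any actor other than its instigator.
; Mesh collision stays off for a brief delay after spawn, then the projectile arms.
; On impact it disarms, turns on gravity, switches collision to ignore pawns and plays an impact sound.
; A separate ApplyDamage function, not called here, line-traces toward a given actor to build hit info for point damage.
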(event `self.ReceiveBeginPlay`
  ; Arm on start
  (set `self.Direction` (`self.GetActorForwardVector`))
  (`PrimitiveComponent.SetCollisionEnabled` (`self.Mesh`) "NoCollision")
  (`KismetSystemLibrary.Delay` 0.025)
  (`PrimitiveComponent.SetCollisionEnabled` (`self.Mesh`) "QueryAndPhysics")
  (set `self.IsArmed` true))

(event `self.ReceiveHit`
  (params (MyComp :type "PrimitiveComponent Object Reference") (Other :type "Actor Object Reference") (OtherComp :type "PrimitiveComponent Object Reference") (bSelfMoved :type Boolean) (HitLocation :type "Vector Structure") (HitNormal :type "Vector Structure") (NormalImpulse :type "Vector Structure") (Hit :type "HitResult Structure (by ref)"))
  (bind _instigator (`self.Instigator`))
  ; Hit Event
  (if (`self.IsArmed`)
    (if (not (== Other _instigator))
      (`GameplayStatics.ApplyPointDamage` Other (`self.Damage`) (`self.Direction`) Hit null _instigator "/Script/Engine.DamageType")
      (set `self.IsArmed` false)
      (set `ProjectileMovementComponent.ProjectileGravityScale` 1.0 (`self.ProjectileMovement`))
      (`PrimitiveComponent.SetCollisionProfileName` (`self.Mesh`) "IgnoreOnlyPawn" false)
      (`GameplayStatics.PlaySoundAtLocation` (`self.ImpactSFX`) (`self.K2_GetActorLocation` self) (struct) 1.0 1.0 0.0 "/Game/CobCop/Audio/AudioSettings/DefaultSoundAttenuation.DefaultSoundAttenuation" null null null))))

(fn `Apply Damage`
  (params (DamagedActor :type "Actor Object Reference"))
  (bind _returnvalue (`self.K2_GetActorLocation`))
  (bind _returnvalue_2 (`self.K2_GetActorLocation` DamagedActor))
  (bind _outhit (`KismetSystemLibrary.LineTraceSingleForObjects` _returnvalue _returnvalue_2 (`|MakeArray` "ObjectTypeQuery1" "ObjectTypeQuery2" "ObjectTypeQuery3" :!type "EObjectTypeQuery Enum") false (`|MakeArray` self :!type "Actor Object Reference")))
  (`GameplayStatics.ApplyPointDamage` DamagedActor (`self.Damage`) (`KismetMathLibrary.Normal` (- _returnvalue_2 _returnvalue)) _outhit null self "/Script/Engine.DamageType"))

(fn `UserConstructionScript`)