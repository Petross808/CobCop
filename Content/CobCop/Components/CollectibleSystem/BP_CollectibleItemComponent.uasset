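; BP_CollectibleItemComponent is an actor component that turns its owning actor into a pickup.
; On BeginPlay it adds a sphere collider to the owner, sized by CollectRadius, and binds its begin-overlap event.
; When an overlapping actor has a BP_CollectorComponent, it fires OnCollected, plays CollectSound in 2D, passes ItemType to that collector and destroys the owner.
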(event `self.ReceiveBeginPlay`
  ; Initialize Collider
  (`|ExecutionSequence`
    (:`then_0`
      (bind _returnvalue (`|AddComponentByClass` :`self` (`self.GetOwner`) :`Class` "/Script/Engine.SphereComponent"))
      (bind _output_get (set `self.Collider` _returnvalue))
      (`SphereComponent.SetSphereRadius` _output_get (`self.CollectRadius`) false))
    (:`then_1`
      (add `PrimitiveComponent.OnComponentBeginOverlap` (`self.Collider`) (delegate `OnCollision`)))))

(event `OnCollision`
  (params (OverlappedComponent :type "PrimitiveComponent Object Reference") (OtherActor :type "Actor Object Reference") (OtherComp :type "PrimitiveComponent Object Reference") (OtherBodyIndex :type Integer) (bFromSweep :type Boolean) (SweepResult :type "HitResult Structure (by ref)"))
  (bind _returnvalue (`Actor.GetComponentByClass` OtherActor "/Game/CobCop/Components/CollectibleSystem/BP_CollectorComponent.BP_CollectorComponent_C"))
  ; Evaluate Collision
  (`/Engine/EditorBlueprintResources/StandardMacros.IsValid` _returnvalue
    (:`Is Valid`
      (`|ExecutionSequence`
        (:`then_0`
          (`self.OnCollected`)
          (`GameplayStatics.PlaySound2D` (`self.CollectSound`) 1.0 1.0 0.0 null null))
        (:`then_1`
          (`/Game/CobCop/Components/CollectibleSystem/BP_CollectorComponent.ItemCollected` _returnvalue (`self.ItemType`)))
        (:`then_2`
          (`Actor.K2_DestroyActor` (`self.GetOwner`)))))))