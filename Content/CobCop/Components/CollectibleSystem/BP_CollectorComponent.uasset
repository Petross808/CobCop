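; Collector component that tracks an owner's collectible totals and inventory items.
; OnCollect adds a collectible's value to its type's count in a map, while unique items live in a set that can be checked and consumed.
; Changes, including ClearAll, are announced through amount-changed, item-collected and item-lost notifications, except SetRaw, which writes amounts silently.
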(event `OnCollect`
  (params (Collectible :type "/Game/CobCop/Components/CollectibleSystem/BP_CollectibleComponent Object Reference"))
  (`self.AddAmount` (`/Game/CobCop/Components/CollectibleSystem/BP_CollectibleComponent.Collectible Type` Collectible) (`/Game/CobCop/Components/CollectibleSystem/BP_CollectibleComponent.Value` Collectible)))

(event `ItemCollected`
  (params (`New Item` :type "/Game/CobCop/Components/CollectibleSystem/E_Items Enum" :default "NewEnumerator0"))
  (`BlueprintSetLibrary.Set_Add` (`self.InventorySet`) `New Item`)
  (`self.OnItemCollected` `New Item`))

(event `ItemLost`
  (params (`Lost Item` :type "/Game/CobCop/Components/CollectibleSystem/E_Items Enum" :default "NewEnumerator0"))
  (`BlueprintSetLibrary.Set_Remove` (`self.InventorySet`) `Lost Item`)
  (`self.OnItemLost` `Lost Item`))

(fn `AddAmount`
  (params (Collectible :type "/Game/CobCop/Components/CollectibleSystem/E_Collectibles Enum" :default "NewEnumerator0") (Amount :type Integer))
  (`self.SetAmount` Collectible (+ (`self.GetAmount` Collectible) Amount)))

(fn `ClearAll`
  (bind _collectiblemap (`self.CollectibleMap`))
  (bind _keypin (`|MapForEach` _collectiblemap)
    (:`then`
      (`self.OnCollectibleAmountChanged` _keypin))
    (:`CompletedPin`
      (`BlueprintMapLibrary.Map_Clear` _collectiblemap)
      (bind _result (`BlueprintSetLibrary.Set_ToArray` (`self.InventorySet`)))
      (for _array_element _result
        (`self.OnItemLost` _array_element))
      (`BlueprintSetLibrary.Set_Clear` (`self.InventorySet`)))))

(fn `GetAmount`
  (params (Collectible :type "/Game/CobCop/Components/CollectibleSystem/E_Collectibles Enum" :default "NewEnumerator0"))
  (returns (Amount :type Integer))
  (bind (_value _returnvalue) (`BlueprintMapLibrary.Map_Find` (`self.CollectibleMap`) Collectible))
  (return (`KismetMathLibrary.SelectInt` _value 0 _returnvalue)))

(fn `SetAmount`
  (params (Collectible :type "/Game/CobCop/Components/CollectibleSystem/E_Collectibles Enum" :default "NewEnumerator0") (Amount :type Integer))
  (`BlueprintMapLibrary.Map_Add` (`self.CollectibleMap`) Collectible Amount)
  (`self.OnCollectibleAmountChanged` Collectible Amount))

(fn `SetRaw`
  (params (Collectible :type "/Game/CobCop/Components/CollectibleSystem/E_Collectibles Enum" :default "NewEnumerator0") (Amount :type Integer))
  (`BlueprintMapLibrary.Map_Add` (`self.CollectibleMap`) Collectible Amount))

(fn `TryConsumeItem`
  (params (Item :type "/Game/CobCop/Components/CollectibleSystem/E_Items Enum" :default "NewEnumerator0"))
  (returns (Success :type Boolean))
  (if (`BlueprintSetLibrary.Set_Contains` (`self.InventorySet`) Item)
    (`self.ItemLost` Item)
    (return true)
    (else
      (return false))))