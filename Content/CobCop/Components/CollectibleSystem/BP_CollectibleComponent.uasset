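; BP_CollectibleComponent is an actor component that turns its owning actor into a pickup for actors carrying a BP_CollectorComponent.
; On BeginPlay it adds a sphere collider sized by CollectRadius and, if SpinSpeed is nonzero, a rotating movement component.
; A valid overlap fires OnCollected, plays CollectSound in 2D and passes itself to the collector's OnCollect.
; It then destroys the owner if DestroyOnCollect is set.
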(event `self.ReceiveBeginPlay`
  ; Initialize Collider
  (`|ExecutionSequence`
    (:`then_0`
      (bind _returnvalue (`|AddComponentByClass` :`self` (`self.GetOwner`) :`Class` "/Script/Engine.SphereComponent"))
      (bind _output_get (set `self.Collider` _returnvalue))
      (`SphereComponent.SetSphereRadius` _output_get (`self.Collect Radius`) false))
    (:`then_1`
      (add `PrimitiveComponent.OnComponentBeginOverlap` (`self.Collider`) (delegate `OnCollision`))
      (`self.SpinSetup`))))

(event `OnCollision`
  (params (OverlappedComponent :type "PrimitiveComponent Object Reference") (OtherActor :type "Actor Object Reference") (OtherComp :type "PrimitiveComponent Object Reference") (OtherBodyIndex :type Integer) (bFromSweep :type Boolean) (SweepResult :type "HitResult Structure (by ref)"))
  (bind _returnvalue (`Actor.GetComponentByClass` OtherActor "/Game/CobCop/Components/CollectibleSystem/BP_CollectorComponent.BP_CollectorComponent_C"))
  ; Evaluate Collision
  (`/Engine/EditorBlueprintResources/StandardMacros.IsValid` _returnvalue
    (:`Is Valid`
      (`|ExecutionSequence`
        (:`then_0`
          (`self.OnCollected` _returnvalue)
          (`GameplayStatics.PlaySound2D` (`self.Collect Sound`) 1.0 1.0 0.0 null null))
        (:`then_1`
          (`/Game/CobCop/Components/CollectibleSystem/BP_CollectorComponent.OnCollect` _returnvalue self))
        (:`then_2`
          (`self.Cleanup`))))))

(event `SpinSetup`
  ; Spin setup
  (if (!= (`self.Spin Speed`) 0.0)
    (bind _returnvalue (`|AddComponentByClass` (`self.GetOwner`) "/Script/Engine.RotatingMovementComponent"))
    (set `RotatingMovementComponent.RotationRate` (`KismetMathLibrary.MakeRotator` 0.0 0.0 (`self.Spin Speed`)) _returnvalue)))

(event `Cleanup`
  ; Default Collect Behaviour
  (if (`self.Destroy on Collect`)
    (`Actor.K2_DestroyActor` (`self.GetOwner`))))