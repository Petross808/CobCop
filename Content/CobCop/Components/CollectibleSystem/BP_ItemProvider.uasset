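; BP_ItemProvider is a component that gives an item, a collectible or both to whoever interacts with its owning actor.
; On BeginPlay it binds to the owner's BP_InteractableComponent interact event.
; The first interaction passes a DoOnce, then looks up BP_CollectorComponent on the interactor's owner.
; If found, the GiveItem and GiveCollectible flags decide whether it calls ItemCollected, AcquireCollectible with an amount, or both.
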(event `self.ReceiveBeginPlay`
  (bind _returnvalue (`Actor.GetComponentByClass` (`self.GetOwner`) "/Game/CobCop/Components/InteractionSystem/BP_InteractableComponent.BP_InteractableComponent_C"))
  (`/Engine/EditorBlueprintResources/StandardMacros.IsValid` _returnvalue
    (:`Is Valid`
      (add `/Game/CobCop/Components/InteractionSystem/BP_InteractableComponent.OnInteract` _returnvalue (delegate `OnInteract_Event`)))))

(event `OnInteract_Event`
  (params (Interactor :type "/Game/CobCop/Components/InteractionSystem/BP_InteractorComponent Object Reference"))
  (bind _returnvalue (`Actor.GetComponentByClass` (`self.GetOwner` Interactor) "/Game/CobCop/Components/CollectibleSystem/BP_CollectorComponent.BP_CollectorComponent_C"))
  (`/Engine/EditorBlueprintResources/StandardMacros.DoOnce` false
    (:`Completed`
      (`/Engine/EditorBlueprintResources/StandardMacros.IsValid` _returnvalue
        (:`Is Valid`
          (`|ExecutionSequence`
            (:`then_0`
              (if (`self.GiveItem`)
                (`/Game/CobCop/Components/CollectibleSystem/BP_CollectorComponent.ItemCollected` _returnvalue (`self.Item`))))
            (:`then_1`
              (if (`self.GiveCollectible`)
                (`/Game/CobCop/Components/CollectibleSystem/BP_CollectorComponent.AcquireCollectible` _returnvalue (`self.Collectible`) (`self.Amount`))))))))))