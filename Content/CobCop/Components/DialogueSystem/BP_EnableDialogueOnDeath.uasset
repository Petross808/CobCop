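; Actor component in the dialogue system that makes a referenced Dialogue's trigger box active only after its owner dies.
; On BeginPlay it disables collision on the Dialogue's BoxCollider and, if the owner has a BP_HealthComponent, binds to that component's OnDeath event.
; When the death event fires, it sets the collider to query and physics collision.
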(event `self.ReceiveBeginPlay`
  (bind _returnvalue (`Actor.GetComponentByClass` (`self.GetOwner`) "/Game/CobCop/Components/CombatSystem/BP_HealthComponent.BP_HealthComponent_C"))
  (`PrimitiveComponent.SetCollisionEnabled` (`/Game/CobCop/Dialogue/BP_TriggerDialogue.BoxCollider` (`self.Dialogue`)) "NoCollision")
  (`/Engine/EditorBlueprintResources/StandardMacros.IsValid` _returnvalue
    (:`Is Valid`
      (add `/Game/CobCop/Components/CombatSystem/BP_HealthComponent.OnDeath` _returnvalue (delegate `OnDeath_Event`)))))

(event `OnDeath_Event`
  (params (`Healt Component` :type "/Game/CobCop/Components/CombatSystem/BP_HealthComponent Object Reference"))
  (`PrimitiveComponent.SetCollisionEnabled` (`/Game/CobCop/Dialogue/BP_TriggerDialogue.BoxCollider` (`self.Dialogue`)) "QueryAndPhysics"))