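; Manager that triggers player and enemy dialogue callouts for attack, hurt, idle and enemy activation moments.
; BeginPlay binds health and attack events on the player and existing enemies, whose handlers roll a chance and check a shared text-length-based cooldown.
; Tick fires idle lines from the nearest enemy in range, otherwise the player.
; Lines come from shuffled arrays, reshuffled when exhausted; GetNextActivationCallout supplies activation lines to callers.
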(event `On Player Attack`
  (params (`Attack Component` :type "/Game/CobCop/Components/CombatSystem/BP_AttackComponent Object Reference"))
  ; Player Attack Callouts
  (if (`KismetMathLibrary.RandomBoolWithWeight` (`self.Attack Callout Chance`)) :!label _label
    (bind _returnvalue (`self.Check Cooldown`))
    (if _returnvalue
      (bind _callout (`self.Get Next Callout` (`self.Player Attack Callouts`) (`self.Player Attack Callouts Index`)))
      (`self.Reset Cooldowns` (`.Text_5_0D12AB694D0A86F579D274BBEDB385FB` (break `/Game/CobCop/Components/DialogueSystem/Callouts/S_CalloutEntry` _callout)))
      (`/Game/CobCop/Components/DialogueSystem/Callouts/BP_Callout.Callout` (`/Game/CobCop/Player/BP_Cornifer.BP_Callout` (`self.Player`)) _callout))))

(event `On Player Shoot`
  (params (`Ranged Attack` :type "/Game/CobCop/Components/CombatSystem/BP_RangedAttack Object Reference"))
  ; Player Attack Callouts
  (goto _label))

(event `self.ReceiveBeginPlay`
  (`|ExecutionSequence`
    (:`then_0`
      ; Get Player
      (bind _returnvalue (`GameplayStatics.GetActorOfClass` "/Game/CobCop/Player/BP_Cornifer.BP_Cornifer_C"))
      (bind _output_get (set `self.Player` _returnvalue))
      ; Player Hurt Callouts
      (add `/Game/CobCop/Components/CombatSystem/BP_HealthComponent.OnDamageEvent` (`/Game/CobCop/Player/BP_Cornifer.Health` _output_get) (delegate `On Player Damaged`))
      ; Player Attack Callouts
      (add `/Game/CobCop/Components/CombatSystem/BP_AttackComponent.On Attack` (`/Game/CobCop/Player/BP_Cornifer.Melee Attack` _output_get) (delegate `On Player Attack`))
      (add `/Game/CobCop/Components/CombatSystem/BP_RangedAttack.On Shoot` (`/Game/CobCop/Player/BP_Cornifer.Ranged Attack` _output_get) (delegate `On Player Shoot`)))
    (:`then_1`
      ; Get all Enemies
      (bind _outactors (`GameplayStatics.GetAllActorsOfClass` "/Game/CobCop/Enemy/BP_EnemyBase.BP_EnemyBase_C"))
      (bind _output_get_2 (set `self.Enemies` _outactors))
      (for _array_element _output_get_2
        (bind _health (`/Game/CobCop/Enemy/BP_EnemyBase.Health` _array_element))
        (add `/Game/CobCop/Components/CombatSystem/BP_HealthComponent.OnDeath` _health (delegate `On Enemy Death`))
        (add `/Game/CobCop/Components/CombatSystem/BP_HealthComponent.OnDamageEvent` _health (delegate `On Enemy Damaged`))
        ; Enemy Attack Callouts
        (bind _asbp_melee_enemy (cast `/Game/CobCop/Enemy/BP_MeleeEnemy` _array_element)
          (:`then`
            (add `/Game/CobCop/Components/CombatSystem/BP_AttackComponent.On Attack` (`/Game/CobCop/Enemy/BP_MeleeEnemy.Melee Attack` _asbp_melee_enemy) (delegate `Enemy Attack`)))
          (:`CastFailed`
            (bind _asbp_ranged_enemy (cast `/Game/CobCop/Enemy/BP_RangedEnemy` _array_element))
            (add `/Game/CobCop/Components/CombatSystem/BP_RangedAttack.On Shoot` (`/Game/CobCop/Enemy/BP_RangedEnemy.RangedAttack` _asbp_ranged_enemy) (delegate `Enemy Shoot`))))))
    (:`then_2`
      (`self.Reset Cooldowns` "")
      (`KismetArrayLibrary.Array_Shuffle` (`self.Enemy Activation Callouts`))
      (`KismetArrayLibrary.Array_Shuffle` (`self.Enemy Idle Callouts`))
      (`KismetArrayLibrary.Array_Shuffle` (`self.Enemy Attack Callouts`))
      (`KismetArrayLibrary.Array_Shuffle` (`self.Enemy Hurt Callouts`))
      (`KismetArrayLibrary.Array_Shuffle` (`self.Player Idle Callouts`))
      (`KismetArrayLibrary.Array_Shuffle` (`self.Player Attack Callouts`))
      (`KismetArrayLibrary.Array_Shuffle` (`self.Player Hurt Callouts`)))))

(event `On Player Damaged`
  (params (`Health Component` :type "/Game/CobCop/Components/CombatSystem/BP_HealthComponent Object Reference"))
  ; Player Hurt Callouts
  (if (`KismetMathLibrary.RandomBoolWithWeight` (`self.Hurt Callout Chance`))
    (bind _returnvalue (`self.Check Cooldown`))
    (if _returnvalue
      (bind _callout (`self.Get Next Callout` (`self.Player Hurt Callouts`) (`self.Player Hurt Callouts Index`)))
      (`self.Reset Cooldowns` (`.Text_5_0D12AB694D0A86F579D274BBEDB385FB` (break `/Game/CobCop/Components/DialogueSystem/Callouts/S_CalloutEntry` _callout)))
      (`/Game/CobCop/Components/DialogueSystem/Callouts/BP_Callout.Callout` (`/Game/CobCop/Player/BP_Cornifer.BP_Callout` (`self.Player`)) _callout))))

(event `Enemy Attack`
  (params (`Attack Component` :type "/Game/CobCop/Components/CombatSystem/BP_AttackComponent Object Reference"))
  ; Enemy Attack Callouts
  (if (`KismetMathLibrary.RandomBoolWithWeight` (`self.Attack Callout Chance`))
    (bind _returnvalue (`self.Check Cooldown`))
    (if _returnvalue
      (bind _asbp_enemy_base (cast `/Game/CobCop/Enemy/BP_EnemyBase` (`ActorComponent.GetOwner` `Attack Component`)))
      (bind _callout (`self.Get Next Callout` (`self.Enemy Attack Callouts`) (`self.Enemy Attack Callouts Index`)))
      (`self.Reset Cooldowns` (`.Text_5_0D12AB694D0A86F579D274BBEDB385FB` (break `/Game/CobCop/Components/DialogueSystem/Callouts/S_CalloutEntry` _callout)))
      (`/Game/CobCop/Components/DialogueSystem/Callouts/BP_Callout.Callout` (`/Game/CobCop/Enemy/BP_EnemyBase.BP_Callout` _asbp_enemy_base) _callout))))

(event `Enemy Shoot`
  (params (`Ranged Attack` :type "/Game/CobCop/Components/CombatSystem/BP_RangedAttack Object Reference"))
  ; Enemy Attack Callouts
  (if (`KismetMathLibrary.RandomBoolWithWeight` (`self.Attack Callout Chance`))
    (bind _returnvalue (`self.Check Cooldown`))
    (if _returnvalue
      (bind _asbp_enemy_base (cast `/Game/CobCop/Enemy/BP_EnemyBase` (`ActorComponent.GetOwner` `Ranged Attack`)))
      (bind _callout (`self.Get Next Callout` (`self.Enemy Attack Callouts`) (`self.Enemy Attack Callouts Index`)))
      (`self.Reset Cooldowns` (`.Text_5_0D12AB694D0A86F579D274BBEDB385FB` (break `/Game/CobCop/Components/DialogueSystem/Callouts/S_CalloutEntry` _callout)))
      (`/Game/CobCop/Components/DialogueSystem/Callouts/BP_Callout.Callout` (`/Game/CobCop/Enemy/BP_EnemyBase.BP_Callout` _asbp_enemy_base) _callout))))

(event `On Enemy Death`
  (params (`Healt Component` :type "/Game/CobCop/Components/CombatSystem/BP_HealthComponent Object Reference"))
  ; Unbind Enemies on Death
  (bind _asbp_enemy_base (cast `/Game/CobCop/Enemy/BP_EnemyBase` (`ActorComponent.GetOwner` `Healt Component`)))
  (`KismetArrayLibrary.Array_RemoveItem` (`self.Enemies`) _asbp_enemy_base))

(event `On Enemy Damaged`
  (params (`Health Component` :type "/Game/CobCop/Components/CombatSystem/BP_HealthComponent Object Reference"))
  ; Enemy Hurt Callouts
  (if (`KismetMathLibrary.RandomBoolWithWeight` (`self.Hurt Callout Chance`))
    (bind _returnvalue (`self.Check Cooldown`))
    (if _returnvalue
      (bind _asbp_enemy_base (cast `/Game/CobCop/Enemy/BP_EnemyBase` (`ActorComponent.GetOwner` `Health Component`)))
      (bind _callout (`self.Get Next Callout` (`self.Enemy Hurt Callouts`) (`self.Enemy Hurt Callouts Index`)))
      (`self.Reset Cooldowns` (`.Text_5_0D12AB694D0A86F579D274BBEDB385FB` (break `/Game/CobCop/Components/DialogueSystem/Callouts/S_CalloutEntry` _callout)))
      (`/Game/CobCop/Components/DialogueSystem/Callouts/BP_Callout.Callout` (`/Game/CobCop/Enemy/BP_EnemyBase.BP_Callout` _asbp_enemy_base) _callout))))

(event `self.ReceiveTick`
  (params (DeltaSeconds :type "Float (single-precision)"))
  (bind (_distance _returnvalue) (`GameplayStatics.FindNearestActor` (`self.K2_GetActorLocation` (`self.Player`)) (`self.Enemies`)))
  ; Cooldown decrease
  (bind _output_get (set `self.Cooldown` (`KismetMathLibrary.FMax` (- (stale _output_get) DeltaSeconds))))
  (bind _output_get_2 (set `self.Idle Cooldown` (`KismetMathLibrary.FMax` (- (stale _output_get_2) DeltaSeconds))))
  ; Idle Callouts
  (if (<= _output_get_2 0.0)
    (if (<= _distance (`self.Min Callout distance`))
      (bind _asbp_enemy_base (cast `/Game/CobCop/Enemy/BP_EnemyBase` _returnvalue))
      (bind _callout (`self.Get Next Callout` (`self.Enemy Idle Callouts`) (`self.Enemy Idle Callouts Index`)))
      (`self.Reset Cooldowns` (`.Text_5_0D12AB694D0A86F579D274BBEDB385FB` (break `/Game/CobCop/Components/DialogueSystem/Callouts/S_CalloutEntry` _callout)))
      (`/Game/CobCop/Components/DialogueSystem/Callouts/BP_Callout.Callout` (`/Game/CobCop/Enemy/BP_EnemyBase.BP_Callout` _asbp_enemy_base) _callout)
      (else
        (bind _callout_2 (`self.Get Next Callout` (`self.Player Idle Callouts`) (`self.Player Idle Callouts Index`)))
        (`self.Reset Cooldowns` (`.Text_5_0D12AB694D0A86F579D274BBEDB385FB` (break `/Game/CobCop/Components/DialogueSystem/Callouts/S_CalloutEntry` _callout_2)))
        (`/Game/CobCop/Components/DialogueSystem/Callouts/BP_Callout.Callout` (`/Game/CobCop/Player/BP_Cornifer.BP_Callout` (`self.Player`)) _callout_2)))))

(fn `Check Cooldown`
  (returns (ReturnValue :type Boolean))
  (locals (ret :type Boolean))
  (return (<= (`self.Cooldown`) 0.0)))

(fn `Get Next Activation Callout`
  (returns (Callout :type "/Game/CobCop/Components/DialogueSystem/Callouts/S_CalloutEntry Structure") (OffCooldown :type Boolean))
  (locals (Ret :type Text) (Success :type Boolean))
  (bind _returnvalue (`self.Check Cooldown`))
  (if _returnvalue
    (bind _callout (`self.Get Next Callout` (`self.Enemy Activation Callouts`) (`self.Enemy Activation Callout index`)))
    (`self.Reset Cooldowns` (`.Text_5_0D12AB694D0A86F579D274BBEDB385FB` (break `/Game/CobCop/Components/DialogueSystem/Callouts/S_CalloutEntry` _callout)))
    (bind _output_get (set `local.Success` true))
    (return _callout _output_get)))

(fn `Get Next Callout`
  (params (Callouts :type "Array of /Game/CobCop/Components/DialogueSystem/Callouts/S_CalloutEntry Structure") (Index :type "Integer (by ref)"))
  (returns (Callout :type "/Game/CobCop/Components/DialogueSystem/Callouts/S_CalloutEntry Structure"))
  (locals (Ret :type "/Game/CobCop/Components/DialogueSystem/Callouts/S_CalloutEntry Structure") (Success :type Boolean))
  (bind _output_get (set `local.Ret` (`|GetArrayItem` Callouts Index)))
  (bind _result (`/Engine/EditorBlueprintResources/StandardMacros.IncrementInt` Index)
    (:`  `
      (if (>= _result (`KismetArrayLibrary.Array_Length` Callouts))
        (`|VariableSetRef` Index)
        (`KismetArrayLibrary.Array_Shuffle` Callouts))
      (return _output_get))))

(fn `Reset Cooldowns`
  (params (Text :type Text))
  (set `self.Cooldown` (+ (/ (`KismetStringLibrary.Len` (`KismetTextLibrary.Conv_TextToString` Text)) (`/Game/CobCop/Components/DialogueSystem/Callouts/BP_GlobalFloat.Value` (`self.Characters per Second`))) (`/Game/CobCop/Components/DialogueSystem/Callouts/BP_GlobalFloat.Value` (`self.Added Delay`))))
  (set `self.Idle Cooldown` (`self.Min Idle Cooldown`)))

(fn `UserConstructionScript`)