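; BP_CalloutTrigger is a box trigger that plays an ordered sequence of dialogue callouts while the player, BP_Cornifer, stands inside it.
; Tick counts down a cooldown based on each line's text length and reading speed plus an added delay, then sends the next entry to its indexed callout displayer.
; It disables itself after the last callout or when a linked actor's interactable component is used.
; The construction script sizes the box from BoxScale.
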(event `self.ReceiveTick`
  (params (DeltaSeconds :type "Float (single-precision)"))
  (bind (_output_calloutdisplayerindex _output_calloutentry) (break `/Game/CobCop/Components/DialogueSystem/Callouts/S_CalloutTriggerEntry` (`|GetArrayItem` (`self.Callouts`) (`self.Index`))))
  (bind _output_get (set `self.Cooldown` (- (stale _output_get) DeltaSeconds)))
  (if (and (<= _output_get 0.0) (stale `self.Box.OnComponentBeginOverlap` _output_get) (`self.Enabled`))
    (set `self.Cooldown` (+ (/ (`KismetStringLibrary.Len` (`KismetTextLibrary.Conv_TextToString` (`.Text_5_0D12AB694D0A86F579D274BBEDB385FB` (break `/Game/CobCop/Components/DialogueSystem/Callouts/S_CalloutEntry` _output_calloutentry)))) (`/Game/CobCop/Components/DialogueSystem/Callouts/BP_GlobalFloat.Value` (`self.Characters per Second`))) (`/Game/CobCop/Components/DialogueSystem/Callouts/BP_GlobalFloat.Value` (`self.Added Delay`))))
    (`/Game/CobCop/Components/DialogueSystem/Callouts/BP_CalloutDisplayer.Play Callout` (`|GetArrayItem` (`self.Callout Displayers`) _output_calloutdisplayerindex) _output_calloutentry)
    (bind _result (`/Engine/EditorBlueprintResources/StandardMacros.IncrementInt` (`self.Index`))
      (:`  `
        (set `self.Enabled` (< _result (`KismetArrayLibrary.Array_Length` (`self.Callouts`))))))))

(event `self.Box.OnComponentBeginOverlap`
  (params (OverlappedComponent :type "PrimitiveComponent Object Reference") (OtherActor :type "Actor Object Reference") (OtherComp :type "PrimitiveComponent Object Reference") (OtherBodyIndex :type Integer) (bFromSweep :type Boolean) (SweepResult :type "HitResult Structure (by ref)"))
  (cast `/Game/CobCop/Player/BP_Cornifer` OtherActor)
  (bind _output_get (set `self.Overlapping Player` true)))

(event `self.Box.OnComponentEndOverlap`
  (params (OverlappedComponent :type "PrimitiveComponent Object Reference") (OtherActor :type "Actor Object Reference") (OtherComp :type "PrimitiveComponent Object Reference") (OtherBodyIndex :type Integer))
  (cast `/Game/CobCop/Player/BP_Cornifer` OtherActor)
  (set `self.Overlapping Player` false))

(event `self.ReceiveBeginPlay`
  (bind _returnvalue (`self.GetComponentByClass` (`self.Interactable to Disable`) "/Game/CobCop/Components/InteractionSystem/BP_InteractableComponent.BP_InteractableComponent_C"))
  (`/Engine/EditorBlueprintResources/StandardMacros.IsValid` _returnvalue
    (:`Is Valid`
      (add `/Game/CobCop/Components/InteractionSystem/BP_InteractableComponent.OnInteract` _returnvalue (delegate `Disable`)))))

(event `Disable`
  (params (Interactor :type "/Game/CobCop/Components/InteractionSystem/BP_InteractorComponent Object Reference"))
  (set `self.Enabled` false))

(fn `UserConstructionScript`
  (`BoxComponent.SetBoxExtent` (`self.Box`) (`self.Box Scale`) true))