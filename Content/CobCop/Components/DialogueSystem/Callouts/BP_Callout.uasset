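; BP_Callout is a dialogue component that shows text callout bubbles over Cornifer or enemies.
; On BeginPlay it finds the callout manager and places a new WBP_CalloutBubble in the owner's widget component.
; The Callout event plays any supplied text in that bubble.
; For enemies, pawn sighting requests an activation line from the manager, playing it if off cooldown and then disabling further aggro callouts.
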(event `self.ReceiveBeginPlay`
  (bind _returnvalue (`self.GetOwner`))
  (bind _returnvalue_2 (`GameplayStatics.GetActorOfClass` "/Game/CobCop/Components/DialogueSystem/Callouts/BP_CalloutManager.BP_CalloutManager_C"))
  (set `self.CalloutManager` _returnvalue_2)
  (bind _asbp_cornifer (cast `/Game/CobCop/Player/BP_Cornifer` _returnvalue)
    (:`then`
      (bind _returnvalue_3 (`|CreateWidget` "/Game/CobCop/Components/DialogueSystem/Callouts/WBP_CalloutBubble.WBP_CalloutBubble_C"))
      (bind _callout_widget (`/Game/CobCop/Player/BP_Cornifer.Callout Widget` _asbp_cornifer))
      (`WidgetComponent.SetWidget` _callout_widget _returnvalue_3)
      (bind _aswbp_callout_bubble (cast `/Game/CobCop/Components/DialogueSystem/Callouts/WBP_CalloutBubble` (`WidgetComponent.GetWidget` _callout_widget)))
      (set `self.Callout Widget` _aswbp_callout_bubble))
    (:`CastFailed`
      (bind _asbp_enemy_base (cast `/Game/CobCop/Enemy/BP_EnemyBase` _returnvalue))
      (bind _returnvalue_4 (`|CreateWidget` "/Game/CobCop/Components/DialogueSystem/Callouts/WBP_CalloutBubble.WBP_CalloutBubble_C"))
      (bind _callout_widget_2 (`/Game/CobCop/Enemy/BP_EnemyBase.Callout Widget` _asbp_enemy_base))
      (`WidgetComponent.SetWidget` _callout_widget_2 _returnvalue_4)
      (bind _aswbp_callout_bubble_2 (cast `/Game/CobCop/Components/DialogueSystem/Callouts/WBP_CalloutBubble` (`WidgetComponent.GetWidget` _callout_widget_2)))
      (set `self.Callout Widget` _aswbp_callout_bubble_2)
      (add `PawnSensingComponent.OnSeePawn` (`/Game/CobCop/Enemy/BP_EnemyBase.PawnSensing` _asbp_enemy_base) (delegate `Aggro Callout`)))))

(event `Callout`
  (params (Text :type Text))
  (bind _output_get (set `self.Text` Text))
  (`/Game/CobCop/Components/DialogueSystem/Callouts/WBP_CalloutBubble.Play` (`self.Callout Widget`) _output_get :!label _label))

(event `Aggro Callout`
  (params (Pawn :type "Pawn Object Reference"))
  (if (`self.Aggro Callout Enabled`)
    (bind (_callout _offcooldown) (`/Game/CobCop/Components/DialogueSystem/Callouts/BP_CalloutManager.Get Next Activation Callout` (`self.CalloutManager`)))
    (if _offcooldown
      (set `self.Text` _callout)
      (set `self.Aggro Callout Enabled` false)
      (goto _label))))