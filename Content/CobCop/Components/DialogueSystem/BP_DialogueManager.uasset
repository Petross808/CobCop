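; Level dialogue manager that advances story dialogue when the player hits key gameplay moments.
; On BeginPlay it binds to the BP_Cornifer collector, first and boss enemy deaths, lock, gate, end door and every Door's teleporter.
; Each handler calls NextDialogue on a referenced dialogue object, with missing-evidence events sharing one.
; Bolt cutter, kernel and missing-key lines are gated by DoOnce, and the first-kill line follows a short delay.
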(event `BoltcutterCollected`
  (params (Item :type "/Game/CobCop/Components/CollectibleSystem/E_Items Enum" :default "NewEnumerator0"))
  (switch `/Game/CobCop/Components/CollectibleSystem/E_Items` Item
    (:`NewEnumerator3`
      (`/Engine/EditorBlueprintResources/StandardMacros.DoOnce` false
        (:`Completed`
          (`/Game/CobCop/Components/DialogueSystem/BP_DialogueComponent.NextDialogue` (`/Game/CobCop/Dialogue/BP_EventDialogue.Dialogue` (`self.BoltcutterDialogue`))))))))

(event `OnCollectibleAmountChanged_Event`
  (params (Collectible :type "/Game/CobCop/Components/CollectibleSystem/E_Collectibles Enum" :default "NewEnumerator0") (`New Amount` :type Integer))
  (switch `/Game/CobCop/Components/CollectibleSystem/E_Collectibles` Collectible
    (:`NewEnumerator0`
      (`/Engine/EditorBlueprintResources/StandardMacros.DoOnce` false
        (:`Completed`
          (`/Game/CobCop/Components/DialogueSystem/BP_DialogueComponent.NextDialogue` (`/Game/CobCop/Dialogue/BP_EventDialogue.Dialogue` (`self.KernelDialogue`))))))))

(event `FirstKill`
  (params (`Healt Component` :type "/Game/CobCop/Components/CombatSystem/BP_HealthComponent Object Reference"))
  (`KismetSystemLibrary.Delay` 0.75)
  (`/Game/CobCop/Components/DialogueSystem/BP_DialogueComponent.NextDialogue` (`/Game/CobCop/Dialogue/BP_EventDialogue.Dialogue` (`self.FirstKillDialogue`))))

(event `self.ReceiveBeginPlay`
  (`|ExecutionSequence`
    (:`then_0`
      (bind _asbp_cornifer (cast `/Game/CobCop/Player/BP_Cornifer` (`GameplayStatics.GetPlayerPawn` 0)))
      (bind _collector (`/Game/CobCop/Player/BP_Cornifer.Collector` _asbp_cornifer))
      (add `/Game/CobCop/Components/CollectibleSystem/BP_CollectorComponent.OnCollectibleAmountChanged` _collector (delegate `OnCollectibleAmountChanged_Event`))
      (add `/Game/CobCop/Components/CollectibleSystem/BP_CollectorComponent.OnItemCollected` _collector (delegate `BoltcutterCollected`)))
    (:`then_1`
      (add `/Game/CobCop/Components/CombatSystem/BP_HealthComponent.OnDeath` (`/Game/CobCop/Enemy/BP_EnemyBase.Health` (`self.FirstEnemy`)) (delegate `FirstKill`)))
    (:`then_2`
      (add `/Game/CobCop/Blueprints_Prefabs/BoltCutterPuzzle/Lock.OnInteractWithoutItem` (`self.Lock`) (delegate `OnInteractWithoutItem_Event`)))
    (:`then_3`
      (add `/Game/CobCop/Components/InteractionSystem/BP_InteractableComponent.OnInteract` (`/Game/CobCop/Blueprints_Prefabs/BoltCutterPuzzle/Gate.BP_InteractableComponent` (`self.Gate`)) (delegate `OnInteract_Event`)))
    (:`then_4`
      (add `/Game/CobCop/Components/CombatSystem/BP_HealthComponent.OnDeath` (`/Game/CobCop/Enemy/BP_EnemyBoss.Health` (`self.BossEnemy`)) (delegate `OnDeath_Event`)))
    (:`then_5`
      (add `/Game/CobCop/Blueprints_Prefabs/Train/EndDoor.InteractWithoutItem` (`self.EndDoor`) (delegate `InteractWithoutKey`)))
    (:`then_6`
      (add `/Game/CobCop/Blueprints_Prefabs/Train/EndDoor.InteractWithoutEvidence` (`self.EndDoor`) (delegate `InteractWithoutEvidence`)))
    (:`then_7`
      (bind _outactors (`GameplayStatics.GetAllActorsOfClass` "/Game/CobCop/Blueprints_Prefabs/Train/Door.Door_C"))
      (for _array_element _outactors
        (add `/Game/CobCop/Components/LevelSystem/ActorTeleporter.OnNotEnoughEvidence` (`/Game/CobCop/Blueprints_Prefabs/Train/Door.ActorTeleporter` _array_element) (delegate `NotEnoughEvidence`))))))

(event `OnInteractWithoutItem_Event`
  (`/Game/CobCop/Components/DialogueSystem/BP_DialogueComponent.NextDialogue` (`/Game/CobCop/Dialogue/BP_EventDialogue.Dialogue` (`self.LockDialogue`))))

(event `OnInteract_Event`
  (params (Interactor :type "/Game/CobCop/Components/InteractionSystem/BP_InteractorComponent Object Reference"))
  (`/Game/CobCop/Components/DialogueSystem/BP_DialogueComponent.NextDialogue` (`/Game/CobCop/Dialogue/BP_EventDialogue.Dialogue` (`self.GateDialogue`))))

(event `OnDeath_Event`
  (params (`Healt Component` :type "/Game/CobCop/Components/CombatSystem/BP_HealthComponent Object Reference"))
  (`/Game/CobCop/Components/DialogueSystem/BP_DialogueComponent.NextDialogue` (`/Game/CobCop/Dialogue/BP_EventDialogue.Dialogue` (`self.BossKillDialogue`))))

(event `InteractWithoutKey`
  (`/Engine/EditorBlueprintResources/StandardMacros.DoOnce` false
    (:`Completed`
      (`/Game/CobCop/Components/DialogueSystem/BP_DialogueComponent.NextDialogue` (`/Game/CobCop/Dialogue/BP_EventDialogue.Dialogue` (`self.EndDoorDialogue`))))))

(event `InteractWithoutEvidence`
  (`/Game/CobCop/Components/DialogueSystem/BP_DialogueComponent.NextDialogue` (`/Game/CobCop/Dialogue/BP_EventDialogue.Dialogue` (`self.NotEnoughEvidenceDialogue`))))

(event `NotEnoughEvidence`
  (`/Game/CobCop/Components/DialogueSystem/BP_DialogueComponent.NextDialogue` (`/Game/CobCop/Dialogue/BP_EventDialogue.Dialogue` (`self.NotEnoughEvidenceDialogue`))))

(fn `UserConstructionScript`)