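; BP_DestructibleComponent makes its owning static-mesh actor shatter the first time it takes point damage.
; On BeginPlay it caches the mesh and materials, then adds a GeometryCollectionComponent with a new GeometryCollection linked to a Dataflow asset.
; On hit it clears the static mesh and evaluates the Dataflow at runtime with mesh, scale and materials overrides.
; It then crumbles the clusters, pushes them along the shot direction with random spin, and plays a sound.
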(event `self.ReceiveBeginPlay`
  (bind _returnvalue (`self.GetOwner`))
  (add `Actor.OnTakePointDamage` _returnvalue (delegate `OnTakePointDamage`))
  (bind _output_get (set `self.SMComponent` (`Actor.GetComponentByClass` _returnvalue "/Script/Engine.StaticMeshComponent")))
  (set `self.Mesh` (`StaticMeshComponent.StaticMesh` _output_get))
  (set `self.Materials` (`MeshComponent.GetMaterials` _output_get))
  (bind _returnvalue_2 (`|AddComponentByClass` :`self` _returnvalue :`Class` "/Script/GeometryCollectionEngine.GeometryCollectionComponent"))
  (bind _output_get_2 (set `self.GCComponent` _returnvalue_2))
  (`PrimitiveComponent.SetCollisionProfileName` _output_get_2 "Destructible" true)
  (bind _returnvalue_3 (`|GenericCreateObject` "/Script/GeometryCollectionEngine.GeometryCollection"))
  (bind _output_get_3 (set `self.GeometryCollection` _returnvalue_3))
  (`GeometryCollection.SetDataflowAsset` _output_get_3 "/Game/CobCop/Destructibles/DestructibleDataflow.DestructibleDataflow"))

(event `OnTakePointDamage`
  (params (DamagedActor :type "Actor Object Reference") (Damage :type "Float (single-precision)") (InstigatedBy :type "Controller Object Reference") (HitLocation :type "Vector Structure") (FHitComponent :type "PrimitiveComponent Object Reference") (BoneName :type Name) (ShotFromDirection :type "Vector Structure") (DamageType :type "DamageType Object Reference") (DamageCauser :type "Actor Object Reference"))
  (if (not (`self.Crumbled`))
    (`StaticMeshComponent.SetStaticMesh` (`self.SMComponent`) null)
    (`GeometryCollectionComponent.SetRestCollection` (`self.GCComponent`) (`self.GeometryCollection`) true)
    (`self.OverrideDataflow` (`GeometryCollectionComponent.RestCollection` (`self.GCComponent`)))
    (`self.Crumble` ShotFromDirection)
    (`GameplayStatics.PlaySoundAtLocation` (`self.Crumble Sound`) (`Actor.K2_GetActorLocation` (`self.GetOwner`)) (struct) 1.0 1.0 0.0 "/Game/CobCop/Audio/DefaultSoundAttenuation.DefaultSoundAttenuation" null null null)))

(fn `Crumble`
  (params (Direction :type "Vector Structure"))
  (bind _gccomponent (`self.GCComponent`))
  (set `self.Crumbled` true)
  (`GeometryCollectionComponent.CrumbleActiveClusters` _gccomponent)
  (`GeometryCollectionComponent.ApplyLinearVelocity` _gccomponent 0 (* Direction 500.0))
  (`GeometryCollectionComponent.ApplyAngularVelocity` _gccomponent 0 (* (`KismetMathLibrary.RandomUnitVector`) 2.0)))

(fn `OverrideDataflow`
  (params (Dataflow :type "Object Object Reference"))
  (bind (_relativescale3d_x _relativescale3d_y _relativescale3d_z) (`KismetMathLibrary.BreakVector` (`SceneComponent.RelativeScale3D` (`self.SMComponent`))))
  (`DataflowBlueprintLibrary.OverrideDataflowVariableObject` Dataflow "Mesh" (`self.Mesh`))
  (`DataflowBlueprintLibrary.OverrideDataflowVariableFloatArray` Dataflow "MeshScale" (`|MakeArray` _relativescale3d_x _relativescale3d_y _relativescale3d_z :!type "Float (single-precision)"))
  (`DataflowBlueprintLibrary.OverrideDataflowVariableObjectArray` Dataflow "Materials" (`self.Materials`))
  (`DataflowBlueprintLibrary.EvaluateTerminalNodeByName` "/Game/CobCop/Destructibles/DestructibleDataflow.DestructibleDataflow" "GeometryCollectionTerminal" Dataflow))