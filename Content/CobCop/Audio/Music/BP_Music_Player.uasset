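; Music player Blueprint that configures a procedural music generator, apparently a MetaSound, for randomized tracks.
; BeginPlay ensures an audio component exists, then calls for a new track.
; The new-track event sets a Quartz clock to a random BPM and sends that tempo, a random key and random scale to the generator as parameters.
; It also enables master, melody, bass, harmony and percussion; gain setters are left unwired.
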(event `self.ReceiveBeginPlay`
  (`/Engine/EditorBlueprintResources/StandardMacros.IsValid` (`self.MSS_MusicGenerator`)
    (:`Is Valid`
      _)
    (:`Is Not Valid`
      (bind _returnvalue (`AddComponent|NODE_AddAudioComponent-1`))
      (set `self.MSS_MusicGenerator` _returnvalue)))
  (`self.New Track`))

(event `New Track_Event`
  (bind _mss_musicgenerator (`self.MSS_MusicGenerator`))
  (bind (_min _max) (break `Int32Interval` (`self.BPM Range`)))
  (`|ExecutionSequence`
    (:`then_0`
      (bind _returnvalue (`QuartzSubsystem.CreateNewClock` :`self` (subsystem `QuartzSubsystem`) :`ClockName` "Clock"))
      (bind _output_get (set `self.QuartzClock` _returnvalue))
      (bind _output_get_2 (set `self.BPM` (`KismetMathLibrary.Conv_IntToDouble` (`KismetMathLibrary.RandomIntegerInRange` _min _max))))
      (`QuartzClockHandle.SetBeatsPerMinute` :`self` _output_get :`BeatsPerMinute` _output_get_2)
      (`AudioComponent.SetFloatParameter` _mss_musicgenerator "BPM" _output_get_2)
      (`AudioComponent.SetFloatParameter` _mss_musicgenerator "Key" (`KismetMathLibrary.Conv_IntToDouble` (+ 54 (`KismetMathLibrary.RandomInteger` 12))))
      (`AudioComponent.SetIntParameter` _mss_musicgenerator "Scale Degrees" (`KismetArrayLibrary.Array_Random` (`self.Scales`))))
    (:`then_1`
      (`AudioComponent.SetBoolParameter` _mss_musicgenerator "Enable Master" true)
      (`AudioComponent.SetBoolParameter` _mss_musicgenerator "Enable Melody" true)
      (`AudioComponent.SetBoolParameter` _mss_musicgenerator "Enable Bass" true)
      (`AudioComponent.SetBoolParameter` _mss_musicgenerator "Enable Harmony" true)
      (`AudioComponent.SetBoolParameter` _mss_musicgenerator "Enable Percussion" true))
    (:`then_2`
      (`AudioParameterControllerInterface.SetObjectParameter` _mss_musicgenerator "None" null))))

(fn `UserConstructionScript`)