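; BP_TrainEngine is a train ambience actor that drives engine and track sounds in response to doors, time and the player camera.
; On BeginPlay it binds every Door's interact event, which fires a "Door" trigger on both sounds.
; A looping 150-second timer, set inside that door loop, triggers a passing-train sound on the tracks.
; Each Tick sets the tracks' "Pan" from the follow camera's Y position and right vector.
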(event `self.ReceiveBeginPlay`
  (bind _asbp_cornifer (cast `/Game/CobCop/Player/BP_Cornifer` (`GameplayStatics.GetPlayerPawn` 0)))
  (bind _output_get (set `self.Follow Camera` (`/Game/CobCop/Player/BP_Cornifer.FollowCamera` _asbp_cornifer)))
  (bind _outactors (`GameplayStatics.GetAllActorsOfClass` "/Game/CobCop/Blueprints_Prefabs/Door.Door_C"))
  (for _array_element _outactors
    (add `/Game/CobCop/Components/InteractionSystem/BP_InteractableComponent.OnInteract` (`/Game/CobCop/Blueprints_Prefabs/Door.Interactable` _array_element) (delegate `OpenDoors`))
    (`KismetSystemLibrary.K2_SetTimerDelegate` (delegate `PassingTrain`) 150.0 true)))

(event `OpenDoors`
  (params (Interactor :type "/Game/CobCop/Components/InteractionSystem/BP_InteractorComponent Object Reference"))
  (`AudioParameterControllerInterface.SetTriggerParameter` (`self.TracksSound`) "Door")
  (`AudioParameterControllerInterface.SetTriggerParameter` (`self.EngineSound`) "Door"))

(event `PassingTrain`
  (`AudioParameterControllerInterface.SetTriggerParameter` (`self.TracksSound`) "TrainPass"))

(event `self.ReceiveTick`
  (params (DeltaSeconds :type "Float (single-precision)"))
  (bind _returnvalue (`SceneComponent.K2_GetComponentToWorld` (stale `self.ReceiveBeginPlay` _output_get)))
  (bind (_returnvalue_x _returnvalue_y) (`KismetMathLibrary.BreakVector` (`KismetMathLibrary.GetRightVector` (.rotation _returnvalue))))
  (`AudioComponent.SetFloatParameter` (`self.TracksSound`) "Pan" (* (/ (.y (.location _returnvalue)) 240.0) _returnvalue_y)))

(fn `UserConstructionScript`)