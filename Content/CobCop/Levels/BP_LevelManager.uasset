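; BP_LevelManager handles level transitions behind a loading screen, loading either a preset level or one passed in by the caller.
; LoadLevel shows the loading screen, waits briefly, async-loads the level asset, then opens it by object reference.
; On BeginPlay it either starts that load immediately or shows the loading screen for a configurable pre-wait time and removes it.
; OpenLevel and OpenCustomLevel events trigger loads on demand.
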(event `self.ReceiveBeginPlay`
  (if (`self.LoadOnStart`)
    (`self.Load Level` (`self.LevelToLoad`) :!label _label)
    (else
      (`UserWidget.AddToViewport` (`self.LoadingScreen`) 500)
      (`KismetSystemLibrary.Delay` (`self.PreWaitTime`))
      (`Widget.RemoveFromParent` (`self.LoadingScreen`)))))

(event `OpenLevel`
  (goto _label))

(event `OpenCustomLevel`
  (params (Level :type "World Soft Object Reference"))
  (`self.Load Level` Level))

(fn `UserConstructionScript`)