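; BP_SoftbodyComponent turns its owning actor into a Chaos Flesh soft body.
; Initialize adds a flesh component, a box overlap volume, a deformable collisions component and a skeletal mesh using the DG_FleshDeformer mesh deformer.
; BeginPlay hides the procedural mesh, feeds static meshes overlapping the box into deformable collisions, and after a delay enables simulation through the level's DeformableSolverActor.
; Tick's vertex-anchored actor repositioning is disabled.
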(event `self.ReceiveEndPlay`
  (params (EndPlayReason :type "EEndPlayReason Enum" :default "Destroyed"))
  (`DeformablePhysicsComponent.DisableSimulation` (`self.FleshComponent`))
  (`DeformablePhysicsComponent.DisableSimulation` (`self.DeformableCollisions`)))

(event `self.ReceiveBeginPlay`
  (bind _collisionvolume (`self.CollisionVolume`))
  (`|ExecutionSequence`
    (:`then_0`
      (bind _output_get (set `self.Mesh` (`Actor.GetComponentByClass` (`self.GetOwner`) "/Script/ProceduralMeshComponent.ProceduralMeshComponent")))
      (`SceneComponent.SetHiddenInGame` _output_get true false))
    (:`then_1`
      (add `PrimitiveComponent.OnComponentBeginOverlap` _collisionvolume (delegate `VolumeBeginOverlap`))
      (add `PrimitiveComponent.OnComponentEndOverlap` _collisionvolume (delegate `VolumeEndOverlap`))
      (bind _outcomponents (`KismetSystemLibrary.ComponentOverlapComponents` _collisionvolume (`SceneComponent.K2_GetComponentToWorld` _collisionvolume) (`|MakeArray` "ObjectTypeQuery1" "ObjectTypeQuery2" :!type "EObjectTypeQuery Enum")))
      (for _array_element _outcomponents
        (bind _asstatic_mesh_component (cast `StaticMeshComponent` _array_element))
        (`DeformableCollisionsComponent.AddStaticMeshComponent` (`self.DeformableCollisions`) _asstatic_mesh_component)))
    (:`then_2`
      (`KismetSystemLibrary.Delay` 1.0)
      (bind _returnvalue (`GameplayStatics.GetActorOfClass` "/Script/ChaosFleshEngine.DeformableSolverActor"))
      (`DeformablePhysicsComponent.EnableSimulationFromActor` (`self.FleshComponent`) _returnvalue)
      (`DeformablePhysicsComponent.EnableSimulationFromActor` (`self.DeformableCollisions`) _returnvalue)
      (set `self.Simulating` true))))

(event `VolumeBeginOverlap`
  (params (OverlappedComponent :type "PrimitiveComponent Object Reference") (OtherActor :type "Actor Object Reference") (OtherComp :type "PrimitiveComponent Object Reference") (OtherBodyIndex :type Integer) (bFromSweep :type Boolean) (SweepResult :type "HitResult Structure (by ref)"))
  (bind _asstatic_mesh_component (cast `StaticMeshComponent` OtherComp))
  (`DeformableCollisionsComponent.AddStaticMeshComponent` (`self.DeformableCollisions`) _asstatic_mesh_component))

(event `VolumeEndOverlap`
  (params (OverlappedComponent :type "PrimitiveComponent Object Reference") (OtherActor :type "Actor Object Reference") (OtherComp :type "PrimitiveComponent Object Reference") (OtherBodyIndex :type Integer))
  (bind _asstatic_mesh_component (cast `StaticMeshComponent` OtherComp))
  (`DeformableCollisionsComponent.RemoveStaticMeshComponent` (`self.DeformableCollisions`) _asstatic_mesh_component))

(event `self.ReceiveTick`
  (params (DeltaSeconds :type "Float (single-precision)"))
  (if false
    (bind _vertices (`KismetProceduralMeshLibrary.GetSectionFromProceduralMesh` (`self.Mesh`)))
    (`Actor.K2_SetActorLocation` (`self.GetOwner`) (`KismetMathLibrary.TransformLocation` (`SceneComponent.K2_GetComponentToWorld` (`self.Mesh`)) (`|GetArrayItem` _vertices (`self.VertexAnchorIndex`))) false false)))

(fn `Initialize`
  (bind _returnvalue (`self.GetOwner`))
  (`|ExecutionSequence`
    (:`then_0`
      (bind _returnvalue_2 (`|AddComponentByClass` :`self` _returnvalue :`Class` "/Script/ChaosFleshEngine.FleshComponent"))
      (bind _output_get (set `self.FleshComponent` _returnvalue_2))
      (`DeformableTetrahedralComponent.SetRestCollection` _output_get (`self.FleshAsset`))
      (`PrimitiveComponent.SetMaterial` _output_get 0 (`self.Material`)))
    (:`then_1`
      (bind _returnvalue_3 (`|AddComponentByClass` :`self` _returnvalue :`Class` "/Script/Engine.BoxComponent"))
      (bind _output_get_2 (set `self.CollisionVolume` _returnvalue_3))
      (`BoxComponent.SetBoxExtent` _output_get_2 (`self.CollisionVolumeSize`) true)
      (set `PrimitiveComponent.bGenerateOverlapEvents` true _output_get_2)
      (`PrimitiveComponent.SetCollisionProfileName` _output_get_2 "OverlapAll" true))
    (:`then_2`
      (bind _returnvalue_4 (`|AddComponentByClass` :`self` _returnvalue :`Class` "/Script/ChaosFleshEngine.DeformableCollisionsComponent"))
      (set `self.DeformableCollisions` _returnvalue_4))
    (:`then_3`
      (bind _returnvalue_5 (`|AddComponentByClass` :`self` _returnvalue :`Class` "/Script/Engine.SkeletalMeshComponent"))
      (`SkeletalMeshComponent.SetSkeletalMeshAsset` _returnvalue_5 (`FleshAsset.SkeletalMesh` (`self.FleshAsset`)))
      (`SkinnedMeshComponent.SetMeshDeformer` _returnvalue_5 "/ChaosFlesh/Deformers/DG_FleshDeformer.DG_FleshDeformer")
      (`PrimitiveComponent.SetMaterial` _returnvalue_5 0 (`self.Material`)))))